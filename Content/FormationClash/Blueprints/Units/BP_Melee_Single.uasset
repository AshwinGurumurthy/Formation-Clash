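; BP_Melee_Single is a unit Blueprint for a single-pattern melee unit in FormationClash.
; On BeginPlay it runs the parent logic, then casts the UnitIcons widget to WBP_UnitIcon and sets its Melee type and Single pattern textures.
; All other behavior comes from the parent class, as the construction script only calls the parent and Tick and overlap events are disabled.
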(event `self.ReceiveBeginPlay`
  (`parent.ReceiveBeginPlay`)
  (bind _aswbp_unit_icon (cast `/Game/FormationClash/Blueprints/WBP_UnitIcon` (`WidgetComponent.GetWidget` (`self.UnitIcons`))))
  (`/Game/FormationClash/Blueprints/WBP_UnitIcon.SetIcons` _aswbp_unit_icon "/Game/FormationClash/Icons/Melee.Melee" "/Game/FormationClash/Icons/Single.Single"))

(fn `UserConstructionScript`
  (`parent.UserConstructionScript`))